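; BP_Projectile is a short-lived projectile actor that moves faster than the player and destroys itself after half a second.
; The Construction Script adds a Projectile Movement component and sets its initial speed to double the ForwardSpeed of the first BP_Player found through Get All Actors Of Class.
; Tick accumulates delta time to handle the lifetime, and the event graph has no overlap or hit logic.
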(event EventBeginPlay)

(event Collision|EventActorBeginOverlap
  (params (OtherActor :type Actor%20Object%20Reference)))

(event EventTick
  (params (DeltaSeconds :type Float%20%28single-precision%29))
  (Variables|Default|SetTime (+ DeltaSeconds (Variables|Default|GetTime)))
  (if (> (Variables|Default|GetTime) 0.5)
    (Actor|DestroyActor)))

(fn ConstructionScript
  (bind _returnvalue (AddComponent|AddProjectileMovementComponent))
  (bind _outactors (Actor|GetAllActorsOfClass "/Game/InfiniteMatrix/Blueprints/BP_Player.BP_Player_C"))
  (Variables|/Script/Engine.ProjectileMovementComponent|SetInitialSpeed _returnvalue (* (Variables|/Game/InfiniteMatrix/Blueprints/BP_Player.BP_Player_C|GetForwardSpeed (Utilities|Array|Get(acopy) _outactors)) 2.0)))